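; Main game player controller, whose only active logic is a debug shortcut for cycling the world through day phases.
; The IA_Debug_AdvanceTime input steps through an array of day-phase Data Layers, wrapping to the first after the last.
; Each step sets the outgoing layer to Loaded rather than Unloaded, then activates the next through the Data Layer Subsystem, non-recursively.
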(event EventBeginPlay)

(event EventTick
  (params (DeltaSeconds :type Float%20%28single-precision%29)))

(event Input|EnhancedActionEvents|EnhancedInputActionIA_Debug_AdvanceTime
  (params (ActionValue :type Boolean) (ElapsedSeconds :type Float%20%28double-precision%29) (TriggeredSeconds :type Float%20%28double-precision%29) (InputAction :type Input%20Action%20Object%20Reference :default "/Game/DinoGame/Input/IA_Debug_AdvanceTime.IA_Debug_AdvanceTime"))
  (CallFunction|DebugCycleDayPhase))

(fn ConstructionScript)

(fn DebugCycleDayPhase
  ;[0 1 0] Deactivate current phase layer:
  (DataLayers|SetDataLayerRuntimeState (WorldSubsystems|GetDataLayerSubsystem) (Utilities|Array|Get(acopy) (Variables|Default|GetDayPhaseLayers) (Variables|Default|GetDayPhaseCurrentIndex)) "Loaded" false :!class /Script/Engine.DataLayerSubsystem)
  ;[0 1 0] Advance to next phase index:
  (Variables|Default|SetDayPhaseCurrentIndex (Math|Integer|SelectInt 0 (+ 1 (Variables|Default|GetDayPhaseCurrentIndex)) (>= (Variables|Default|GetDayPhaseCurrentIndex) (- (Utilities|Array|Length (Variables|Default|GetDayPhaseLayers)) 1))))
  ;[0 1 0] Activate next phase layer:
  (DataLayers|SetDataLayerRuntimeState (WorldSubsystems|GetDataLayerSubsystem) (Utilities|Array|Get(acopy) (Variables|Default|GetDayPhaseLayers) (Variables|Default|GetDayPhaseCurrentIndex)) "Activated" false :!class /Script/Engine.DataLayerSubsystem))