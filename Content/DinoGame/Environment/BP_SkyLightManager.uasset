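; BP_SkyLightManager positions the sun and moon lights for the game's day phases.
; SetLightRotations takes a phase index and sets each valid light's pitch from its own per-phase array, keeping roll and yaw.
; The rotation is applied instantly, and a call to play the day-phase transition sequence sits unconnected in the event graph.
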(fn ConstructionScript)

(fn SetLightRotations
  (params (RotationIndex :type Integer))
  (bind _sunlight_ref (Variables|Default|GetSunLight_Ref))
  (bind _moonlight_ref (Variables|Default|GetMoonLight_Ref))
  (bind _returnvalue (Transformation|GetActorRotation _moonlight_ref))
  (bind _returnvalue_2 (Transformation|GetActorRotation _sunlight_ref))
  (Utilities|FlowControl|Sequence
    (:then_0
      ;[0 1 0] Set sun angle:
      (Utilities|IsValid _sunlight_ref
        (:Is%20Valid
          (Transformation|SetActorRotation _sunlight_ref (Math|Rotator|MakeRotator (.roll _returnvalue_2) (Utilities|Array|Get(acopy) (Variables|Default|GetDayPhaseSunRotationValues) RotationIndex) (.yaw _returnvalue_2))))))
    (:then_1
      ;[0 1 0] Set moon angle:
      (Utilities|IsValid _moonlight_ref
        (:Is%20Valid
          (Transformation|SetActorRotation _moonlight_ref (Math|Rotator|MakeRotator (.roll _returnvalue) (Utilities|Array|Get(acopy) (Variables|Default|GetDayPhaseMoonRotationValues) RotationIndex) (.yaw _returnvalue))))))
    (:then_2
      (return))))